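; Master Blueprint for breakable resource nodes that give the player inventory items when damaged and destroyed.
; Each TakeDamage event caches player 0's inventory, lowers Health and adds a small random amount of RecievedItem without notification.
; When Health reaches zero, Break grants a larger random amount and destroys the actor only if that add succeeds.
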(event Custom|TakeDamage
  (params (Damage :type Float%20%28single-precision%29))
  (bind _asplayer (Utilities|Casting|CastToPlayer (Game|GetPlayerCharacter 0)))
  (Variables|Default|SetInventory (Variables|/Game/Player/Player.Player_C|GetInventoryRef _asplayer))
  (Variables|Default|SetHealth (- (Variables|Default|GetHealth) Damage))
  (Default|AddItem (Variables|Default|GetInventory) (Variables|Default|GetRecievedItem) (Math|Random|RandomIntegerinRange 1 2) false)
  (if (<= (Variables|Default|GetHealth) 0.0)
    (CallFunction|Break)))

(event Custom|Break
  (bind _success_ (Default|AddItem (Variables|Default|GetInventory) (Variables|Default|GetRecievedItem) (Math|Random|RandomIntegerinRange 2 5) false))
  (if _success_
    (Actor|DestroyActor)))

(fn ConstructionScript)