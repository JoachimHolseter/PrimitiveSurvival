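; World pickup actor that gives an inventory item to the player.
; The construction script takes mesh, scale, offset and interaction radius from the item class defaults, and a widget shows name and amount.
; Sphere overlaps maintain the player's list of nearby pickups, showing text only for the first.
; PickUpItem adds to the inventory, records the remainder by ID in LootedPickups, and either keeps the leftover or destroys the actor.
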(event OnComponentBeginOverlap(Sphere)
  (params (OverlappedComponent :type Primitive%20Component%20Object%20Reference) (OtherActor :type Actor%20Object%20Reference) (OtherComp :type Primitive%20Component%20Object%20Reference) (OtherBodyIndex :type Integer) (bFromSweep :type Boolean) (SweepResult :type Hit%20Result%20Structure%20%28by%20ref%29))
  (bind _asplayer (Utilities|Casting|CastToPlayer OtherActor))
  (if (> (Utilities|Array|Length (Variables|/Game/Player/Player.Player_C|GetNearbyPickupActors _asplayer)) 0)
    (Utilities|Array|Add (Variables|/Game/Player/Player.Player_C|GetNearbyPickupActors _asplayer) self)
    (else
      (Rendering|SetVisibility (Variables|Default|GetPickupText) true false)
      (Utilities|Array|Add (Variables|/Game/Player/Player.Player_C|GetNearbyPickupActors _asplayer) self))))

(event OnComponentEndOverlap(Sphere)
  (params (OverlappedComponent :type Primitive%20Component%20Object%20Reference) (OtherActor :type Actor%20Object%20Reference) (OtherComp :type Primitive%20Component%20Object%20Reference) (OtherBodyIndex :type Integer))
  (bind _asplayer (Utilities|Casting|CastToPlayer OtherActor))
  (if (and (Utilities|IsValid (Utilities|Array|Get(acopy) (Variables|/Game/Player/Player.Player_C|GetNearbyPickupActors _asplayer))) (== (Utilities|Array|Get(acopy) (Variables|/Game/Player/Player.Player_C|GetNearbyPickupActors _asplayer)) self))
    (Rendering|SetVisibility (Variables|Default|GetPickupText) false false)
    (Utilities|Array|RemoveItem (Variables|/Game/Player/Player.Player_C|GetNearbyPickupActors _asplayer) self)
    (Utilities|IsValid (Utilities|Array|Get(acopy) (Variables|/Game/Player/Player.Player_C|GetNearbyPickupActors _asplayer))
      (:Is%20Valid
        (Rendering|SetVisibility (Variables|BP_PickupActor_C|GetPickupText (Utilities|Array|Get(acopy) (Variables|/Game/Player/Player.Player_C|GetNearbyPickupActors _asplayer))) true false)))
    (else
      (Utilities|Array|RemoveItem (Variables|/Game/Player/Player.Player_C|GetNearbyPickupActors _asplayer) self))))

(event Custom|PickUpItem
  (params (Player :type Player%20Object%20Reference))
  (bind _inventoryref (Variables|/Game/Player/Player.Player_C|GetInventoryRef Player))
  (bind _inventoryref_2 (Variables|/Game/Player/Player.Player_C|GetInventoryRef Player))
  (bind _nearbypickupactors (Variables|/Game/Player/Player.Player_C|GetNearbyPickupActors Player))
  (bind _output (Utilities|Array|Get(acopy) _nearbypickupactors))
  (Utilities|IsValid _inventoryref_2
    (:Is%20Valid
      (bind (_success_ _rest_) (Default|AddItem _inventoryref_2 (Variables|Default|GetItemToAdd) (Variables|Default|GetAmount) false))
      (if _success_
        (if (> _rest_ 0)
          (Variables|Default|SetAmount _rest_)
          (CallFunction|UpdateText)
          (Utilities|Array|Add (Variables|/Game/InventorySystem/Blueprints/BP_Inventory.BP_Inventory_C|GetLootedPickups _inventoryref) (Utilities|Struct|MakeS_SavedPickup (Variables|Default|GetID) (Variables|Default|GetAmount)))
          (else
            (Utilities|Array|Add (Variables|/Game/InventorySystem/Blueprints/BP_Inventory.BP_Inventory_C|GetLootedPickups _inventoryref) (Utilities|Struct|MakeS_SavedPickup (Variables|Default|GetID) 0))
            (Utilities|Array|RemoveItem _nearbypickupactors self)
            (Utilities|IsValid _output
              (:Is%20Valid
                (Rendering|SetVisibility (Variables|BP_PickupActor_C|GetPickupText _output) true false)
                (Actor|DestroyActor))
              (:Is%20Not%20Valid
                (Actor|DestroyActor)))))))))

(event EventBeginPlay
  (CallFunction|UpdateText))

(fn ConstructionScript
  (bind _itemtoadd (Variables|Default|GetItemToAdd))
  (bind _mesh (Variables|Default|GetMesh))
  (bind _mesh_2 (Variables|Default|GetMesh))
  (bind _iteminfo (Utilities|GetClassDefaults _itemtoadd))
  (bind (_name _description _icon _canbeused_ _usetext _canbestacked _category _internalname _weight _recipe _hasdurability_ _durability _pickupmesh _meshscale _meshoffset _interactradius) (Utilities|Struct|BreakS_ItemInfo _iteminfo))
  (if (Utilities|IsValidClass _itemtoadd)
    (Components|StaticMesh|SetStaticMesh _mesh _pickupmesh)
    (Variables|Default|SetOriginalMaterial (Rendering|Material|GetMaterial _mesh 0))
    (Transformation|SetRelativeScale3D _mesh _meshscale)
    (Components|Sphere|SetSphereRadius (Variables|Default|GetSphere) _interactradius false)
    (Transformation|SetRelativeLocation _mesh_2 (+ (Variables|/Script/Engine.SceneComponent|GetRelativeLocation _mesh_2) _meshoffset) false false)))

(fn UpdateText
  (bind _itemtoadd (Variables|Default|GetItemToAdd))
  (bind _amount (Variables|Default|GetAmount))
  (bind _iteminfo (Utilities|GetClassDefaults _itemtoadd))
  (bind _name (Utilities|Struct|BreakS_ItemInfo _iteminfo))
  (bind _aspickup_text (Utilities|Casting|CastToPickupText (UserInterface|GetUserWidgetObject (Variables|Default|GetPickupText)))
    (:then
      (Rendering|Components|TextRender|SetText (Variables|/Game/InventorySystem/Widgets/PickupText.PickupText_C|GetNametext _aspickup_text) (select (== _amount 1) _name (Utilities|Text|FormatText "{Name} ({Amount})" _name _amount))))
    (:CastFailed
      _))
  (return))