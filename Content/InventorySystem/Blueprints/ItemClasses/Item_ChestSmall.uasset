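; Inventory item class for a small chest that places a chest in the world when used.
; On use it spawns BP_ChestSmall at a random positive X and Y offset from the player's capsule, at a fixed height, ignoring collisions.
; It then removes one of itself from the inventory slot and destroys its own actor.
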(event EventBeginPlay)

(event Collision|EventActorBeginOverlap
  (params (OtherActor :type Actor%20Object%20Reference)))

(event EventTick
  (params (DeltaSeconds :type Float%20%28single-precision%29)))

(event EventEventonUsed
  (bind _asplayer (Utilities|Casting|CastToPlayer (Game|GetPlayerCharacter 0)))
  (Game|SpawnActorfromClass "/Game/InventorySystem/Blueprints/BP_ChestSmall.BP_ChestSmall_C" (Math|Transform|MakeTransform (Math|Vector|MakeVector (+ (.x (Transformation|GetWorldLocation (Variables|/Script/Engine.Character|GetCapsuleComponent _asplayer))) (Math|Random|RandomFloatinRange 7e+01 1e+02)) (+ (.y (Transformation|GetWorldLocation (Variables|/Script/Engine.Character|GetCapsuleComponent _asplayer))) (Math|Random|RandomFloatinRange 7e+01 1e+02)) -35.0) "0, 0, 0" "1,1,1") "AlwaysSpawn" 0 30 10 0)
  (Default|RemoveItematIndex (Variables|Default|GetInventory) (Variables|Default|GetIndex) 1)
  (Actor|DestroyActor))

(fn ConstructionScript
  (|CallParentFunction))