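; Sandwich item class for the inventory system, a consumable food that restores the player's hunger when used.
; On use, it checks the player's hunger through the inventory's player reference and, if below maximum, adds its food amount and removes one unit from its inventory slot.
; The item actor destroys itself after use, including when hunger is already full and nothing is consumed.
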(event EventBeginPlay
  (|CallParentFunction) ; This node is disabled and will not be called.\nDrag off pins to build functionality.
)

(event Collision|EventActorBeginOverlap
  (params (OtherActor :type Actor%20Object%20Reference))
  (|CallParentFunction OtherActor) ; This node is disabled and will not be called.\nDrag off pins to build functionality.
)

(event EventTick
  (params (DeltaSeconds :type Float%20%28single-precision%29))
  (|CallParentFunction DeltaSeconds) ; This node is disabled and will not be called.\nDrag off pins to build functionality.
)

(event EventEventonUsed
  (bind _inventory (Variables|Default|GetInventory))
  (bind _playerreference (Variables|/Game/InventorySystem/Blueprints/BP_Inventory.BP_Inventory_C|GetPlayerReference _inventory))
  (if (< (Variables|/Game/Player/Player.Player_C|GetHunger _playerreference) (Variables|/Game/Player/Player.Player_C|GetMaxHunger _playerreference))
    (Default|AddHunger _playerreference (Variables|Default|GetFoodAmount))
    (Default|RemoveItematIndex (Variables|Default|GetInventory) (Variables|Default|GetIndex) 1)
    (Actor|DestroyActor)
    (else
      (Actor|DestroyActor))))

(fn ConstructionScript
  (|CallParentFunction))