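; Small storage chest that players open to access its own slot-based inventory.
; Range overlap toggles the prompt text and registers the chest as the player's NearbyChest.
; Interacting passes a DoOnce, lazily spawns and reuses a BP_Storage actor, shows storage and inventory, hides crafting, and switches to UI input with movement disabled.
; Closing storage restores game input and walking, then resets the DoOnce for the next interaction.
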(event OnComponentBeginOverlap(Range)
  (params (OverlappedComponent :type Primitive%20Component%20Object%20Reference) (OtherActor :type Actor%20Object%20Reference) (OtherComp :type Primitive%20Component%20Object%20Reference) (OtherBodyIndex :type Integer) (bFromSweep :type Boolean) (SweepResult :type Hit%20Result%20Structure%20%28by%20ref%29))
  (bind _asplayer (Utilities|Casting|CastToPlayer OtherActor))
  (Rendering|SetVisibility (Variables|Default|GetChestText) true false)
  (Variables|/Game/Player/Player.Player_C|SetNearbyChest _asplayer self))

(event OnComponentEndOverlap(Range)
  (params (OverlappedComponent :type Primitive%20Component%20Object%20Reference) (OtherActor :type Actor%20Object%20Reference) (OtherComp :type Primitive%20Component%20Object%20Reference) (OtherBodyIndex :type Integer))
  (bind _asplayer (Utilities|Casting|CastToPlayer OtherActor))
  (Rendering|SetVisibility (Variables|Default|GetChestText) false false)
  (Variables|/Game/Player/Player.Player_C|SetNearbyChest _asplayer 0))

(event Custom|OnStorageClosed
  (bind _returnvalue (Game|GetPlayerController 0))
  (bind _returnvalue_2 (Game|GetPlayerController 0))
  (Default|HideStorage (Variables|Default|GetStorageActor))
  (Input|SetInputModeGameOnly _returnvalue_2)
  (Variables|/Script/Engine.PlayerController|SetbShowMouseCursor _returnvalue_2 false)
  (Pawn|Components|CharacterMovement|SetMovementMode (Variables|/Script/Engine.Character|GetCharacterMovement (Variables|Default|GetPlayer)) "MOVE_Walking" 0)
  (if (Variables|/Game/InventorySystem/Blueprints/BP_Inventory.BP_Inventory_C|GetisVisible? (Variables|/Game/Player/Player.Player_C|GetInventoryRef (Variables|Default|GetPlayer)))
    (Default|HideInventory (Variables|/Game/Player/Player.Player_C|GetInventoryRef (Variables|Default|GetPlayer)))
    (Default|ShowInventory (Variables|/Game/Player/Player.Player_C|GetInventoryRef (Variables|Default|GetPlayer)))
    (Utilities|FlowControl|DoOnce false) ; enters at Reset
    (else
      (Utilities|FlowControl|DoOnce false) ; enters at Reset
    )))

(event Custom|OnInteract
  (params (Player :type Player%20Object%20Reference))
  (bind _returnvalue (Game|GetPlayerController 0))
  (Utilities|FlowControl|DoOnce false
    (:Completed
      (Variables|Default|SetPlayer Player)
      (Widget|SetVisibility (Variables|/Game/InventorySystem/Widgets/MainWidget.MainWidget_C|GetCraftingMenu (Variables|/Game/InventorySystem/Blueprints/BP_Inventory.BP_Inventory_C|GetMainWidget (Variables|/Game/Player/Player.Player_C|GetInventoryRef (Variables|Default|GetPlayer)))) "Hidden")
      (Input|SetInputModeUIOnly _returnvalue 0 "DoNotLock")
      (Variables|/Script/Engine.PlayerController|SetbShowMouseCursor _returnvalue true)
      (Utilities|IsValid (Variables|Default|GetStorageActor)
        (:Is%20Valid
          _)
        (:Is%20Not%20Valid
          (bind _returnvalue_2 (Game|SpawnActorfromClass "/Game/InventorySystem/Blueprints/BP_Storage.BP_Storage_C" (Math|Transform|MakeTransform "0, 0, 0" "0, 0, 0" "1,1,1") "AlwaysSpawn" 0 (Variables|Default|GetAmountOfSlots) (Variables|Default|GetPlayer) (Variables|Default|GetSlotsPerRow) self 0))
          (Variables|Default|SetStorageActor _returnvalue_2)))
      (Default|GenerateSlotWidgets (Variables|/Game/InventorySystem/Blueprints/BP_Storage.BP_Storage_C|GetStorageWidget (Variables|Default|GetStorageActor)) (Variables|Default|GetStorageActor))
      (Default|ShowStorage (Variables|Default|GetStorageActor))
      (Default|HideInventory (Variables|/Game/Player/Player.Player_C|GetInventoryRef (Variables|Default|GetPlayer)))
      (Default|ShowInventory (Variables|/Game/Player/Player.Player_C|GetInventoryRef (Variables|Default|GetPlayer)))
      (Pawn|Components|CharacterMovement|DisableMovement (Variables|/Script/Engine.Character|GetCharacterMovement (Variables|Default|GetPlayer)))
      (Components|Movement|StopMovementImmediately (Variables|/Script/Engine.Character|GetCharacterMovement (Variables|Default|GetPlayer))))))

(fn ConstructionScript)